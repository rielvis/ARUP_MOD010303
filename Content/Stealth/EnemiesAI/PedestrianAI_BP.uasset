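; Pedestrian AI pawn that patrols a looping route through its TargetPoints array.
; From BeginPlay, AIMoveTo moves the pawn to the current point; on success it advances or wraps the index, waits briefly and moves again.
; Only successful moves continue the loop, as failure is unhandled.
; The PawnSensing sight event is empty, and leftover speed-change and player stealth-kill overlap nodes are disconnected.
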(event `self.ReceiveBeginPlay`
  (bind _targetpoints (`self.TargetPoints`))
  ;[1 1 1] Enemy_AI petrolling
  (`|AIMoveTo` (`PawnMovementComponent.GetPawnOwner` (`self.FloatingPawnMovement`)) (0.0 0.0 0.0) (`|GetArrayItem` _targetpoints (`self.TargetPointCount`)) 10.0 :!label _label
    (:`OnSuccess`
      (if (== (`KismetArrayLibrary.Array_LastIndex` _targetpoints) (`self.TargetPointCount`))
        (set `self.TargetPointCount` 0)
        (else
          (set `self.TargetPointCount` (+ (`self.TargetPointCount`) 1))))
      (`KismetSystemLibrary.Delay` 1.0)
      (goto _label))))

(event `self.PawnSensing.OnSeePawn`
  (params (Pawn :type "Pawn Object Reference")))

(fn `UserConstructionScript`)