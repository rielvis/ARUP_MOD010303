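; Knife-wielding stealth enemy character that the player can take down from front or back, then drag and drop.
; Interface events from outside drive the vision cone colour, alert bar and melee animation; melee damage is only a debug print.
; Front and back overlap boxes set the player's kill flags, with the front also alerting the controller.
; Takedown tags the enemy Dead, unpossesses it and enables dragging by attachment, with a downward trace placing dropped bodies.
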(event `self.ReceiveBeginPlay`
  ;[1 1 1] Event Begin Play
  (`/Game/Stealth/ThirdPersonBP/Blueprints/ThirdPersonCharacter.Event_StealthKillOverlap` (cast `/Game/Stealth/ThirdPersonBP/Blueprints/ThirdPersonCharacter` (`GameplayStatics.GetPlayerCharacter` 0) :!pure true) self)
  (bind _outactors (`GameplayStatics.GetAllActorsOfClass` "/Game/Stealth/BPActors/StealthHideActor_BP.StealthHideActor_BP_C"))
  (for (_array_element _array_index) _outactors
    (`KismetArrayLibrary.Array_Set` (`self.HideActor_Ref`) _array_index _array_element true)))

(event `Event_AlertStatus`
  (params (AlertBarFloat :type "Float (double-precision)"))
  ;[1 1 1] Updating AlertBar Widget Value
  (bind _aswidget_alert_status (cast `/Game/Stealth/ThirdPersonBP/Blueprints/Widget_AlertStatus` (`WidgetComponent.GetWidget` (`self.Widget_AlertBar`))))
  (`ProgressBar.SetPercent` (`/Game/Stealth/ThirdPersonBP/Blueprints/Widget_AlertStatus.AlertBar` _aswidget_alert_status) AlertBarFloat))

(event `/Game/Stealth/EnemiesAI/EnemiesAI_Knife/ICombat_Interface.IVisionConeColour`
  (params (ConeColour :type String))
  ;[1 1 1] Vision Cone Colours w.r.t Alert States
  (`KismetSystemLibrary.PrintString` ConeColour true true (struct :`R` 0.115812 :`G` 1.0 :`A` 1.0))
  (switch `string` ConeColour
    (:`Green`
      (`PrimitiveComponent.SetMaterial` (`self.StaticMesh_VisionCone`) 0 "/Game/Stealth/Materials/Cone_Green_Inst.Cone_Green_Inst"))
    (:`Yellow`
      (`PrimitiveComponent.SetMaterial` (`self.StaticMesh_VisionCone`) 0 "/Game/Stealth/Materials/Cone_Yellow_Inst.Cone_Yellow_Inst"))
    (:`Orange`
      (`PrimitiveComponent.SetMaterial` (`self.StaticMesh_VisionCone`) 0 "/Game/Stealth/Materials/Cone_Orange_Inst.Cone_Orange_Inst"))
    (:`Red`
      (`PrimitiveComponent.SetMaterial` (`self.StaticMesh_VisionCone`) 0 "/Game/Stealth/Materials/Cone_Red_Inst.Cone_Red_Inst"))))

(event `/Game/Stealth/EnemiesAI/EnemiesAI_Knife/ICombat_Interface.IMeleeAttack_Function`
  ;[1 1 1] Melee Attack when in range of our character
  (`SkeletalMeshComponent.PlayAnimation` (`self.Mesh`) "/Game/Animations/Zlorp/ZlorpAttack_Hand_Enemy.ZlorpAttack_Hand_Enemy" false)
  (`KismetSystemLibrary.PrintString` "melee attack"))

(event `self.Box_Back.OnComponentBeginOverlap`
  (params (OverlappedComponent :type "PrimitiveComponent Object Reference") (OtherActor :type "Actor Object Reference") (OtherComp :type "PrimitiveComponent Object Reference") (OtherBodyIndex :type Integer) (bFromSweep :type Boolean) (SweepResult :type "HitResult Structure (by ref)"))
  ;[1 1 1] Overlap box on back of enemy to get stealth kill (Back_Box_Overlap)
  (bind _asthird_person_character (cast `/Game/Stealth/ThirdPersonBP/Blueprints/ThirdPersonCharacter` OtherActor))
  (`/Game/Stealth/ThirdPersonBP/Blueprints/ThirdPersonCharacter.Event_TargetEnemyReference` _asthird_person_character "EnemyCharacterKnife_BP_C" self)
  (set `/Game/Stealth/ThirdPersonBP/Blueprints/ThirdPersonCharacter.InBackStealthKillBox?` true _asthird_person_character)
  (set `self.LocalInBackStealthKillBox?` true))

(event `self.Box_MeleeAttackDamage.OnComponentBeginOverlap`
  (params (OverlappedComponent :type "PrimitiveComponent Object Reference") (OtherActor :type "Actor Object Reference") (OtherComp :type "PrimitiveComponent Object Reference") (OtherBodyIndex :type Integer) (bFromSweep :type Boolean) (SweepResult :type "HitResult Structure (by ref)"))
  ;[1 1 1] Melee Attack when in range of our character
  (cast `/Game/Stealth/ThirdPersonBP/Blueprints/ThirdPersonCharacter` OtherActor)
  (`/Engine/EditorBlueprintResources/StandardMacros.DoOnce` false :!label _label
    (:`Completed`
      (`KismetSystemLibrary.PrintString` "DamageApplied" true true (struct :`R` 1.0 :`G` 0.144344 :`A` 1.0))
      (`KismetSystemLibrary.Delay` 1.5)
      (goto _label :!via `Reset`))))

(event `self.Box_Back.OnComponentEndOverlap`
  (params (OverlappedComponent :type "PrimitiveComponent Object Reference") (OtherActor :type "Actor Object Reference") (OtherComp :type "PrimitiveComponent Object Reference") (OtherBodyIndex :type Integer))
  ;[1 1 1] Overlap box on back of enemy to get stealth kill (Back_Box_Overlap)
  ;;[1 1 1] End Collision to Disable Can Take Down
  (bind _asthird_person_character (cast `/Game/Stealth/ThirdPersonBP/Blueprints/ThirdPersonCharacter` OtherActor))
  (set `/Game/Stealth/ThirdPersonBP/Blueprints/ThirdPersonCharacter.InBackStealthKillBox?` false _asthird_person_character)
  (set `self.LocalInBackStealthKillBox?` false))

(event `/Game/Stealth/ThirdPersonBP/Blueprints/ICallToEnemy.ICheckInBackStealthKillBox?`
  ;[1 1 1] Overlap box on back of enemy to get stealth kill (Back_Box_Overlap)
  ;;[1 1 1] COnfirmation. Is in back stealth kill box?
  (bind _asthird_person_character (cast `/Game/Stealth/ThirdPersonBP/Blueprints/ThirdPersonCharacter` (`GameplayStatics.GetPlayerCharacter` 0)))
  (`/Game/Stealth/ThirdPersonBP/Blueprints/ThirdPersonCharacter.Event_BackStealthKillBox?` _asthird_person_character (`self.LocalInBackStealthKillBox?`)))

(event `/Game/Stealth/ThirdPersonBP/Blueprints/ICallToEnemy.IDesiredEnemyToTakedown`
  (params (`FrontKillAnimPlay?` :type Boolean))
  (bind _returnvalue (`self.GetController`))
  ;[1 1 1] Stealth Kill animation run and disabling movement
  (`KismetSystemLibrary.PrintString` (`KismetStringLibrary.Conv_BoolToString` `FrontKillAnimPlay?`) true true (struct :`R` 1.0 :`G` 0.082829 :`A` 1.0))
  (if `FrontKillAnimPlay?`
    (set `self.Front Kill Anim Play?` `FrontKillAnimPlay?`) ; For animation
    (else
      (set `self.BackStealthKill_Anim` true)))
  (`CharacterMovementComponent.DisableMovement` (`self.CharacterMovement`))
  (`KismetArrayLibrary.Array_Set` (`self.Tags`) 0 "Dead" true) ; dead tag at index 0 bcoz hidden/unhidden is on 1
  (`ActorComponent.K2_DestroyComponent` (`self.StaticMesh_VisionCone`))
  (`ActorComponent.K2_DestroyComponent` (`self.Widget_AlertBar`))
  (message `/Game/Stealth/EnemiesAI/EnemiesAI_Rifle/IEnemyRifleToAI_Interface.IEnemyRifle_ControllerDeath` _returnvalue)
  (`Controller.UnPossess` _returnvalue)
  (set `self.CanDrag?` true) ; Enemy is killed now you can drag him
  (set `self.IsDead` true)
  (`PrimitiveComponent.SetCollisionResponseToChannel` (`self.CapsuleComponent`) "ECC_Pawn" "ECR_Ignore"))

(event `Event_GetStealthAttack`
  (params (KillBool :type Boolean))
  ;[1 1 1] Get Stealth kill and anim bool
  (bind _output_get (set `self.BackStealthKill_Anim` KillBool)))

(event `/Game/Stealth/ThirdPersonBP/Blueprints/ICallToEnemy.IHiddenUnhiddenTag`
  (params (Tag :type Name))
  ;[1 1 1] Enemy Hidden Unhidden Tag Tag at index 1
  (`KismetArrayLibrary.Array_Set` (`self.Tags`) 1 Tag true))

(event `self.Box_Front.OnComponentBeginOverlap`
  (params (OverlappedComponent :type "PrimitiveComponent Object Reference") (OtherActor :type "Actor Object Reference") (OtherComp :type "PrimitiveComponent Object Reference") (OtherBodyIndex :type Integer) (bFromSweep :type Boolean) (SweepResult :type "HitResult Structure (by ref)"))
  ;[1 1 1] Enemy Too CLose From Front
  (bind _asthird_person_character (cast `/Game/Stealth/ThirdPersonBP/Blueprints/ThirdPersonCharacter` OtherActor))
  (message `/Game/Stealth/EnemiesAI/EnemiesAI_Knife/IEnemyKnifeToAI_Interface.IEnemyKnifeTooCLose` (`self.GetController`))
  (set `/Game/Stealth/ThirdPersonBP/Blueprints/ThirdPersonCharacter.InFrontKillBox?` true _asthird_person_character))

(event `self.Box_Front.OnComponentEndOverlap`
  (params (OverlappedComponent :type "PrimitiveComponent Object Reference") (OtherActor :type "Actor Object Reference") (OtherComp :type "PrimitiveComponent Object Reference") (OtherBodyIndex :type Integer))
  ;[1 1 1] Enemy Too CLose From Front
  (bind _asthird_person_character (cast `/Game/Stealth/ThirdPersonBP/Blueprints/ThirdPersonCharacter` OtherActor))
  (set `/Game/Stealth/ThirdPersonBP/Blueprints/ThirdPersonCharacter.InFrontKillBox?` false _asthird_person_character))

(event `/Game/Stealth/ThirdPersonBP/Blueprints/ICallToEnemy.IDragBody`
  (params (`DesiredEnemy ` :type "Character Object Reference") (DragCOllisionBox :type "SceneComponent Object Reference") (`InStealthKillBox?` :type Boolean))
  ;[1 1 1] Body Drag only when in Box Front back collision boxes after killing enemy
  (if (`self.CanDrag?`)
    (`PrimitiveComponent.SetCollisionEnabled` (`self.CapsuleComponent`) "NoCollision")
    (`self.K2_AttachToComponent` `DesiredEnemy ` DragCOllisionBox "None" "SnapToTarget" "KeepWorld" "KeepWorld" true)
    (else
      (`KismetSystemLibrary.PrintString` "InBox"))))

(event `/Game/Stealth/ThirdPersonBP/Blueprints/ICallToEnemy.IDragBodyDrop`
  (params (BodyToDrop :type "Character Object Reference"))
  (bind _returnvalue (`self.K2_GetActorLocation` (`GameplayStatics.GetPlayerCharacter` 0)))
  ;[1 1 1] Dropping lifted body. Detaching
  (if (`self.CanDrag?`)
    (bind _outhit (`KismetSystemLibrary.LineTraceSingle` _returnvalue (+ _returnvalue (0.0 0.0 -500.0)) "TraceTypeQuery1" false (`self.HideActor_Ref`) "Persistent"))
    (`self.K2_SetActorLocation` BodyToDrop (+ (`.ImpactPoint` (`GameplayStatics.BreakHitResult` _outhit)) (0.0 0.0 100.0)) true false)
    (`self.K2_DetachFromActor` BodyToDrop "KeepWorld" "KeepWorld" "KeepWorld")
    (`KismetSystemLibrary.Delay` 0.5)
    (`PrimitiveComponent.SetCollisionEnabled` (`self.CapsuleComponent`) "QueryAndProbe")
    (`PrimitiveComponent.SetCollisionEnabled` (`self.Mesh`) "QueryAndProbe")
    (else
      (`KismetSystemLibrary.PrintString` "Cant Drag Body Bcoz Enemy is alive"))))

(fn `UserConstructionScript`)