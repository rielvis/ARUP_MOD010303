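; Objective system Blueprint that steps the player through an ordered array of objective update actors.
; On BeginPlay, after a short delay for HUD loading, it sends the first objective to the third-person character's mission HUD and messages the current objective actor through interface calls.
; A custom event increments the index and notifies the next actor, without a bounds check, printing the index for debugging.
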(event `self.ReceiveBeginPlay`
  (bind _currentobjectivenumber (`self.CurrentObjectiveNumber`))
  (bind _output (`|GetArrayItem` (`self.ObjectiveUpdate_Array_Ref`) _currentobjectivenumber))
  (`KismetSystemLibrary.Delay` 1.0) ; Delay so that HUD is first loaded in TP person then we calling here
  (bind _asthird_person_character (cast `/Game/Stealth/ThirdPersonBP/Blueprints/ThirdPersonCharacter` (`GameplayStatics.GetPlayerCharacter` 0)))
  (set `self.MissionHUD_Ref` (`/Game/Stealth/ThirdPersonBP/Blueprints/ThirdPersonCharacter.MissionHUD_Ref` _asthird_person_character))
  (message `/Game/Stealth/ThirdPersonBP/Blueprints/IObjective_Interface.IObjective_Update_toHUD` (`self.MissionHUD_Ref`) (`self.Objective`)) ; Sending FIrst Objective to Mission HUD
  ;[1 1 1] Sending Current Objective details to Objective Update_BP.
  (message `/Game/Stealth/ThirdPersonBP/Blueprints/IObjective_Interface.IObjectiveUpdate` _output _output _currentobjectivenumber)
  (`KismetSystemLibrary.PrintString` (`KismetSystemLibrary.GetDisplayName` _output) true true (struct :`A` 1.0)))

(event `Event_UpdaeNextObjective`
  (bind _currentobjectivenumber (`self.CurrentObjectiveNumber`))
  (bind _output (`|GetArrayItem` (`self.ObjectiveUpdate_Array_Ref`) _currentobjectivenumber))
  ;[1 1 1] Sending Details to NExt ObjectiveUpdate collider by Fetching Next entry from Objective_Update_Array_Ref
  (set `self.CurrentObjectiveNumber` (+ (`self.CurrentObjectiveNumber`) 1))
  (message `/Game/Stealth/ThirdPersonBP/Blueprints/IObjective_Interface.IObjectiveUpdate` _output _output _currentobjectivenumber)
  (`KismetSystemLibrary.PrintString` (`KismetStringLibrary.Conv_IntToString` (`self.CurrentObjectiveNumber`))))

(fn `UserConstructionScript`)