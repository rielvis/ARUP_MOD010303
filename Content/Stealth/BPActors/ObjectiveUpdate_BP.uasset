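; Objective checkpoint actor for missions, completed by the player entering its box or, for interactive objectives, pressing interact while inside.
; Collision stays off until IObjectiveUpdate enables it, reveals the marker widget and passes objective details to ThirdPersonCharacter.
; Completion sends the objective to the mission HUD, then has ObjectiveSystem_BP advance and destroys the previous checkpoint after a short delay.
; The last objective only prints "Mission Complete"; a DoOnce guards against repeated overlaps.
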(event `self.ReceiveBeginPlay`
  (`PrimitiveComponent.SetCollisionEnabled` (`self.Box_ObjectiveUpdate`) "NoCollision") ; Setting collision disabled. So that only that objectiveUpdate works which is currently active
  (`KismetSystemLibrary.Delay` 1.0) ; Putting Delay so that we can pulling data from Tp Person
  (bind _asthird_person_character (cast `/Game/Stealth/ThirdPersonBP/Blueprints/ThirdPersonCharacter` (`GameplayStatics.GetPlayerCharacter` 0)))
  (set `self.MissionHUD_Ref` (`/Game/Stealth/ThirdPersonBP/Blueprints/ThirdPersonCharacter.MissionHUD_Ref` _asthird_person_character)))

(event `/Game/Stealth/ThirdPersonBP/Blueprints/IObjective_Interface.IObjectiveUpdate`
  (params (CurrentObjectiveActor_Ref :type "Actor Object Reference") (CurrentObjectiveNumber :type Integer))
  ;[1 1 1] Setting Current ObjectiveUPdate collider active by activating its collision, Marker Widget Unhidden and sending ccurrent objective details to TP person To use in case of interactive objectives
  (`SceneComponent.SetHiddenInGame` (`self.Widget`) false false)
  (`KismetSystemLibrary.PrintString` "Objective update recieved" true true (struct :`R` 1.0 :`G` 0.311977 :`A` 1.0))
  (`PrimitiveComponent.SetCollisionEnabled` (`self.Box_ObjectiveUpdate`) "QueryOnly")
  (bind _asthird_person_character (cast `/Game/Stealth/ThirdPersonBP/Blueprints/ThirdPersonCharacter` (`GameplayStatics.GetPlayerCharacter` 0)))
  (`/Game/Stealth/ThirdPersonBP/Blueprints/ThirdPersonCharacter.Event_RecieveObjectiveUpdate` _asthird_person_character CurrentObjectiveActor_Ref CurrentObjectiveNumber))

(event `/Game/Stealth/ThirdPersonBP/Blueprints/IObjective_Interface.IInteractObjective`
  ;[1 1 1] PressTouch/Button to interact with objective. Only works for interactive type objectives. And it will work only when TP person is in ObjectiveUpdatecollision box
  (if (`self.Overlapped?`)
    (`KismetSystemLibrary.PrintString` "Touch screen Recieved" true true (struct :`R` 0.208912 :`G` 1.0 :`B` 0.113665 :`A` 1.0))
    (message `/Game/Stealth/ThirdPersonBP/Blueprints/IObjective_Interface.IObjective_Update_toHUD` (`self.MissionHUD_Ref`) (`self.Objective`) :!label _label) ; Sending Upates to Mission HUD to display
    (`KismetSystemLibrary.PrintString` "Objective overlapped")
    ;[1 1 1] If all objectives are completed then mission complete screen will popup. Otherwise continue with next objective using Event Update Next Objective and destroying current objective update collider so that TpPerson cant overlap it again
    (bind _asobjective_system_bp (castclass `/Game/Stealth/BPActors/ObjectiveSystem_BP` "/Game/Stealth/BPActors/ObjectiveSystem_BP.ObjectiveSystem_BP_C"))
    (bind _returnvalue (`GameplayStatics.GetActorOfClass` _asobjective_system_bp))
    (bind _objectiveupdate_array_ref (`/Game/Stealth/BPActors/ObjectiveSystem_BP.ObjectiveUpdate_Array_Ref` _returnvalue))
    (bind _returnvalue_2 (`KismetArrayLibrary.Array_LastIndex` _objectiveupdate_array_ref))
    (bind _currentobjectivenumber (`/Game/Stealth/BPActors/ObjectiveSystem_BP.CurrentObjectiveNumber` _returnvalue))
    (if (== _returnvalue_2 _currentobjectivenumber)
      (`KismetSystemLibrary.PrintString` "Mission Complete" true true (struct :`G` 1.0 :`B` 0.163426 :`A` 1.0))
      (else
        (`/Game/Stealth/BPActors/ObjectiveSystem_BP.Event_UpdaeNextObjective` _returnvalue)
        (`KismetSystemLibrary.Delay` 0.2)
        (`self.K2_DestroyActor` (`|GetArrayItem` _objectiveupdate_array_ref (`KismetMathLibrary.Clamp` (- _currentobjectivenumber 1) 0 _returnvalue_2)))))))

(event `self.Box_ObjectiveUpdate.OnComponentBeginOverlap`
  (params (OverlappedComponent :type "PrimitiveComponent Object Reference") (OtherActor :type "Actor Object Reference") (OtherComp :type "PrimitiveComponent Object Reference") (OtherBodyIndex :type Integer) (bFromSweep :type Boolean) (SweepResult :type "HitResult Structure (by ref)"))
  ;[1 1 1] Overlapping with ThirdPersonCharacter
  (cast `/Game/Stealth/ThirdPersonBP/Blueprints/ThirdPersonCharacter` OtherActor)
  (`/Engine/EditorBlueprintResources/StandardMacros.DoOnce` false :!label _label_2 ; using it to avoid multiple collision bug
    (:`Completed`
      (set `self.Overlapped?` true)
      (if (`self.InteractiveObjective?`)
        (`KismetSystemLibrary.PrintString` "Touch Screen to Complete Objective" true true (struct :`R` 1.0 :`B` 0.034584 :`A` 1.0) 5.0)
        (message `/Game/Stealth/ThirdPersonBP/Blueprints/IObjective_Interface.INotifications` (`self.MissionHUD_Ref`) "Press Interact Button to Complete Objective") ; Sending to MissionHUD
        (else
          (goto _label))))))

(event `self.Box_ObjectiveUpdate.OnComponentEndOverlap`
  (params (OverlappedComponent :type "PrimitiveComponent Object Reference") (OtherActor :type "Actor Object Reference") (OtherComp :type "PrimitiveComponent Object Reference") (OtherBodyIndex :type Integer))
  (cast `/Game/Stealth/ThirdPersonBP/Blueprints/ThirdPersonCharacter` OtherActor)
  (set `self.Overlapped?` false)
  (goto _label_2 :!via `Reset`))

(fn `UserConstructionScript`)