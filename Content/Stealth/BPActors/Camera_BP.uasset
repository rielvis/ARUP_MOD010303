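; Security camera actor for a stealth game that sweeps its view and raises an alarm when it detects the player.
; An optional timeline drives the camera's yaw, and the construction script places the vision cone mesh from exposed transform variables.
; Player overlap with the cone reports an "Alarm" noise event for enemies.
; Clicking or touching the camera while the player is inside the hack box destroys the cone, stops rotation and tilts it down.
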(event `self.ReceiveBeginPlay`
  (bind (_relativerotation_roll _relativerotation_pitch) (`KismetMathLibrary.BreakRotator` (`SceneComponent.RelativeRotation` (`self.SM_Camera`))))
  ;[1 1 1] Regular Camera Rotation
  (if (`self.CameraRotation?`)
    (bind (_direction _cameraangle) (`Timeline|Timeline_CameraRotation` :!via `PlayFromStart`)
      (:`Update`
        (`SceneComponent.K2_SetRelativeRotation` (`self.SM_Camera`) (`KismetMathLibrary.MakeRotator` _relativerotation_roll _relativerotation_pitch _cameraangle) false false)))))

(event `self.SM_VisionCone.OnComponentBeginOverlap`
  (params (OverlappedComponent :type "PrimitiveComponent Object Reference") (OtherActor :type "Actor Object Reference") (OtherComp :type "PrimitiveComponent Object Reference") (OtherBodyIndex :type Integer) (bFromSweep :type Boolean) (SweepResult :type "HitResult Structure (by ref)"))
  ;[1 1 1] Alarm Alert to enemies when our character detects by camera range
  (bind _asthird_person_character (cast `/Game/Stealth/ThirdPersonBP/Blueprints/ThirdPersonCharacter` OtherActor))
  (`AISense_Hearing.ReportNoiseEvent` (`SceneComponent.K2_GetComponentLocation` (`self.DefaultSceneRoot`)) 1.0 _asthird_person_character 0.0 "Alarm")
  (`KismetSystemLibrary.PrintString` "Hello"))

(event `self.SM_Camera.OnClicked`
  (params (TouchedComponent :type "PrimitiveComponent Object Reference") (ButtonPressed :type "Key Structure"))
  (bind (_relativerotation_roll _relativerotation_pitch _relativerotation_yaw) (`KismetMathLibrary.BreakRotator` (`SceneComponent.RelativeRotation` (`self.SM_Camera`))))
  ;[1 1 1] Camera Hack on Camera Touch
  (if (`self.CanHackCamera?`) :!label _label
    (`ActorComponent.K2_DestroyComponent` (`self.SM_VisionCone`))
    (`TimelineComponent.Stop` (`self.Timeline_CameraRotation`))
    (`SceneComponent.K2_SetRelativeRotation` (`self.SM_Camera`) (`KismetMathLibrary.MakeRotator` _relativerotation_roll -60.0 _relativerotation_yaw) false false)
    (else
      (`KismetSystemLibrary.PrintString` "Camera Out Of Range" true true (struct :`R` 1.0 :`G` 0.025803 :`A` 1.0)))))

(event `self.SM_Camera.OnInputTouchBegin`
  (params (FingerIndex :type "ETouchIndex Enum" :default "Touch1") (TouchedComponent :type "PrimitiveComponent Object Reference"))
  ;[1 1 1] Camera Hack on Camera Touch
  (goto _label))

(event `self.Box_CameraHackArea.OnComponentBeginOverlap`
  (params (OverlappedComponent :type "PrimitiveComponent Object Reference") (OtherActor :type "Actor Object Reference") (OtherComp :type "PrimitiveComponent Object Reference") (OtherBodyIndex :type Integer) (bFromSweep :type Boolean) (SweepResult :type "HitResult Structure (by ref)"))
  ;[1 1 1] Is character in camera hack area?
  (cast `/Game/Stealth/ThirdPersonBP/Blueprints/ThirdPersonCharacter` OtherActor)
  (set `self.CanHackCamera?` true))

(event `self.Box_CameraHackArea.OnComponentEndOverlap`
  (params (OverlappedComponent :type "PrimitiveComponent Object Reference") (OtherActor :type "Actor Object Reference") (OtherComp :type "PrimitiveComponent Object Reference") (OtherBodyIndex :type Integer))
  ;[1 1 1] Is character in camera hack area?
  (cast `/Game/Stealth/ThirdPersonBP/Blueprints/ThirdPersonCharacter` OtherActor)
  (set `self.CanHackCamera?` false))

(fn `UserConstructionScript`
  (`SceneComponent.K2_SetRelativeTransform` (`self.SM_VisionCone`) (`KismetMathLibrary.MakeTransform` (`self.Camera_Vision_Location`) (`self.Camera_Vision_Rotation`) (`self.Camera_Vision_Scale`)) false false))