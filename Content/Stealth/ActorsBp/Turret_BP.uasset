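; Stealth-game turret that raises an alarm and fires when the player enters its vision cone, and can be hacked.
; Cone overlap turns it red, reports an "Alarm" noise and starts a delayed fire loop that randomly hits about half the time until overlap ends.
; Touching the turret while the player is inside the hack box destroys the cone.
; The Construction Script positions the hack box from transform variables.
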(event `Event_TurretStartFiring`
  ;[1 1 1] Turret Fire. If player gets in vision cone turret will start firing
  (`GameplayStatics.PlaySound2D` "/Game/Stealth/SFX/Explosion01.Explosion01" 1.0 1.0 0.0 null null :!label _label)
  (`GameplayStatics.SpawnEmitterAttached` "/Game/Stealth/Particles/P_Explosion1.P_Explosion1" (`self.SM_Turret`))
  (switch `int` (`KismetMathLibrary.RandomIntegerInRange` 1 8)
    (:`0`
      _)
    (:`1`
      (`/Game/Stealth/ThirdPersonBP/Blueprints/ThirdPersonCharacter.Event_TurretFire` (cast `/Game/Stealth/ThirdPersonBP/Blueprints/ThirdPersonCharacter` (`GameplayStatics.GetPlayerCharacter` 0) :!pure true) :!label _label_2))
    (:`2`
      _)
    (:`3`
      (goto _label_2))
    (:`4`
      _)
    (:`5`
      (goto _label_2))
    (:`6`
      _)
    (:`7`
      (goto _label_2))
    (:`8`
      _))
  (`KismetSystemLibrary.Delay` (`self.TurretFireRate`))
  (if (not (`self.OutOfRange?`))
    (goto _label)))

(event `self.Box_HackArea_Turret.OnComponentBeginOverlap`
  (params (OverlappedComponent :type "PrimitiveComponent Object Reference") (OtherActor :type "Actor Object Reference") (OtherComp :type "PrimitiveComponent Object Reference") (OtherBodyIndex :type Integer) (bFromSweep :type Boolean) (SweepResult :type "HitResult Structure (by ref)"))
  ;[1 1 1] Hack Area. Hack available if player gets in hack box
  (cast `/Game/Stealth/ThirdPersonBP/Blueprints/ThirdPersonCharacter` OtherActor)
  (set `self.CanHackTurret?` true)
  (`KismetSystemLibrary.PrintString` "In Hack Area"))

(event `self.SM_VisionCone_Turret.OnComponentEndOverlap`
  (params (OverlappedComponent :type "PrimitiveComponent Object Reference") (OtherActor :type "Actor Object Reference") (OtherComp :type "PrimitiveComponent Object Reference") (OtherBodyIndex :type Integer))
  ;[1 1 1] Turret Vision COne. Set Alarm if player gets in Vision cone area
  (cast `/Game/Stealth/ThirdPersonBP/Blueprints/ThirdPersonCharacter` OtherActor)
  (`PrimitiveComponent.SetMaterial` (`self.SM_VisionCone_Turret`) 0 "/Game/Stealth/Materials/Cone_Green_Inst.Cone_Green_Inst")
  (set `self.OutOfRange?` true))

(event `self.Box_HackArea_Turret.OnComponentEndOverlap`
  (params (OverlappedComponent :type "PrimitiveComponent Object Reference") (OtherActor :type "Actor Object Reference") (OtherComp :type "PrimitiveComponent Object Reference") (OtherBodyIndex :type Integer))
  ;[1 1 1] Hack Area. Hack available if player gets in hack box
  (cast `/Game/Stealth/ThirdPersonBP/Blueprints/ThirdPersonCharacter` OtherActor)
  (set `self.CanHackTurret?` false))

(event `self.SM_VisionCone_Turret.OnComponentBeginOverlap`
  (params (OverlappedComponent :type "PrimitiveComponent Object Reference") (OtherActor :type "Actor Object Reference") (OtherComp :type "PrimitiveComponent Object Reference") (OtherBodyIndex :type Integer) (bFromSweep :type Boolean) (SweepResult :type "HitResult Structure (by ref)"))
  ;[1 1 1] Turret Vision COne. Set Alarm if player gets in Vision cone area
  (bind _asthird_person_character (cast `/Game/Stealth/ThirdPersonBP/Blueprints/ThirdPersonCharacter` OtherActor))
  (`AISense_Hearing.ReportNoiseEvent` (`self.K2_GetActorLocation`) 1.0 _asthird_person_character 0.0 "Alarm")
  (`self.Event_TurretStartFiring`)
  (`PrimitiveComponent.SetMaterial` (`self.SM_VisionCone_Turret`) 0 "/Game/Stealth/Materials/Cone_Red_Inst.Cone_Red_Inst")
  (set `self.OutOfRange?` false))

(event `self.SM_Turret.OnInputTouchBegin`
  (params (FingerIndex :type "ETouchIndex Enum" :default "Touch1") (TouchedComponent :type "PrimitiveComponent Object Reference"))
  ;[1 1 1] Hack Turret
  (if (`self.CanHackTurret?`)
    (`ActorComponent.K2_DestroyComponent` (`self.SM_VisionCone_Turret`))
    (`KismetSystemLibrary.PrintString` "Turret Hacked")
    (else
      (`KismetSystemLibrary.PrintString` "Turret Out Of Range" true true (struct :`R` 1.0 :`G` 0.025803 :`A` 1.0)))))

(fn `UserConstructionScript`
  (`SceneComponent.K2_SetRelativeTransform` (`self.Box_HackArea_Turret`) (`KismetMathLibrary.MakeTransform` (`self.Turret_HackArea_Location`) (`self.Turret_HackArea_Rotation`) (`self.Turret_HackArea_Scale`)) false false))