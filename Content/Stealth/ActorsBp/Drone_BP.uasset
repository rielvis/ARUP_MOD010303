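; Player-controlled scouting drone pawn for the stealth game, steered by planar movement axes and touch-swipe look.
; BeginPlay blends the camera to the drone and caches the ThirdPersonCharacter and mission HUD.
; Forward-axis input checks distance to the character; leaving range starts a HUD warning countdown, which returning cancels.
; Timer expiry, the DroneActive action or the TouchDrone interface repossesses the character, forces crouch and destroys the drone.
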(event `InputTouch`
  (params (Location :type "Vector Structure") (FingerIndex :type "ETouchIndex Enum"))
  (bind _returnvalue (`Controller.K2_GetPawn` (`GameplayStatics.GetPlayerController` 0)))
  (bind (_locationx _locationy) (`PlayerController.GetInputTouchState` (`GameplayStatics.GetPlayerController` 0) FingerIndex))
  (bind _returnvalue_2 (`KismetMathLibrary.MakeVector2D` _locationx _locationy))
  (bind (_returnvalue_x _returnvalue_y) (`KismetMathLibrary.BreakVector2D` (* (- _returnvalue_2 (`self.PriorLoc`)) (`self.SwipeSpeed`))))
  ;[1 1 1] Swipe Touch Control
  (:`Pressed`
    (bind _output_get (set `self.StartLoc` _returnvalue_2))
    (set `self.PriorLoc` _output_get)
    (goto _label :!via `Open`))
  (:`Released`
    (goto _label :!via `Close`))
  (:`Moved`
    (`|ExecutionSequence`
      (:`then_0`
        (`/Engine/EditorBlueprintResources/StandardMacros.Gate` true :!label _label
          (:`Exit`
            (if (>= (`KismetMathLibrary.VSize2D` (- _returnvalue_2 _output_get)) (`self.SwipeThreshold`))
              (set `self.StartLoc` (1000000.0 1000000.0))
              (`self.AddControllerYawInput` _returnvalue _returnvalue_x)
              (`self.AddControllerPitchInput` _returnvalue _returnvalue_y)
              (set `self.PriorLoc` _returnvalue_2)))))
      (:`then_1`
        (`KismetSystemLibrary.PrintString` (`KismetStringLibrary.Conv_DoubleToString` _locationx))))))

(event `Event_Touch_Drone`)

(event `/Game/Stealth/ThirdPersonBP/Blueprints/ITouchHUD.ITouch_Drone`
  (bind _thirdpersoncharacter_ref (`self.ThirdPersonCharacter_Ref`))
  ;[1 1 1] Posessing our character back Pressing R
  (`Controller.Possess` (`GameplayStatics.GetPlayerController` 0) _thirdpersoncharacter_ref :!label _label_2)
  (`KismetSystemLibrary.Delay` 0.2)
  (`Character.Crouch` _thirdpersoncharacter_ref) ; When controller posessess character again It is be default in stand positiion. So forcing crouch here
  (set `/Game/Stealth/ThirdPersonBP/Blueprints/ThirdPersonCharacter.Crouch_Anim` true _thirdpersoncharacter_ref)
  (`self.K2_DestroyActor`))

(event `InputAction|DroneActive`
  (params (Key :type "Key Structure"))
  ;[1 1 1] Posessing our character back Pressing R
  (:`Pressed`
    (goto _label_2)))

(event `InputTouch`
  (params (Location :type "Vector Structure") (FingerIndex :type "ETouchIndex Enum")))

(event `Event_PossessTPActor`
  (goto _label_2))

(event `self.ReceiveBeginPlay`
  ;[1 1 1] Event Begin Play
  (`PlayerController.SetViewTargetWithBlend` (`GameplayStatics.GetPlayerController` 0) self 1.0 "VTBlend_Linear" 0.0 false)
  (bind _asthird_person_character (cast `/Game/Stealth/ThirdPersonBP/Blueprints/ThirdPersonCharacter` (`GameplayStatics.GetPlayerCharacter` 0)))
  (set `self.ThirdPersonCharacter_Ref` _asthird_person_character)
  (set `self.Mission HUD Ref` (`/Game/Stealth/ThirdPersonBP/Blueprints/ThirdPersonCharacter.MissionHUD_Ref` _asthird_person_character)))

(event `InputAxis|MoveForward` :overrideparent false
  (params (AxisValue :type "Float (single-precision)"))
  (bind _returnvalue (`self.GetDistanceTo` (`self.ThirdPersonCharacter_Ref`)))
  ;[1 1 1] Drone Movement (W,A,S,D)
  (`self.AddMovementInput` (`KismetMathLibrary.GetForwardVector` (`KismetMathLibrary.MakeRotator` 0.0 0.0 (.yaw (`self.GetControlRotation`)))) (* AxisValue 0.3))
  ;[1 1 1] Drone to Character distance check and Limit
  (if (> _returnvalue 1200.0)
    (`/Engine/EditorBlueprintResources/StandardMacros.DoOnce` false :!label _label_3
      (:`Completed`
        (`KismetSystemLibrary.PrintString` "Drone Max Distance Reached")
        (`KismetSystemLibrary.Delay` 0.5)
        (bind _returnvalue_2 (`KismetSystemLibrary.K2_SetTimerDelegate` (delegate `Timer`) 1.0 true 1.0))
        (set `self.DroneTimerHandler` _returnvalue_2)
        (message `/Game/Stealth/ThirdPersonBP/Blueprints/IObjective_Interface.INotifications` (`self.Mission HUD Ref`) "Drone Max Distance Reached") ; Sending to MissionHUD
      ))
    (else
      (`|ExecutionSequence`
        (:`then_0`
          (`KismetSystemLibrary.K2_ClearAndInvalidateTimerHandle` (`self.DroneTimerHandler`))
          (set `self.DroneTImer` 6) ; Reseting Timer
        )
        (:`then_1`
          (`KismetSystemLibrary.PrintString` (`KismetStringLibrary.Conv_DoubleToString` _returnvalue) false))
        (:`then_2`
          (goto _label_3 :!via `Reset`))))))

(event `Timer`
  (set `self.DroneTImer` (`KismetMathLibrary.Clamp` (- (`self.DroneTImer`) 1) 0 5))
  (`KismetSystemLibrary.PrintString` (`KismetStringLibrary.Conv_IntToString` (`self.DroneTImer`)))
  (if (<= (`self.DroneTImer`) 0)
    ;[1 1 1] Drone out of zone
    (`self.Event_PossessTPActor`) ; If Drone Timer Becomes zero then call this event to unpossess drone and possess TPCharacter
    (else
      (message `/Game/Stealth/ThirdPersonBP/Blueprints/IObjective_Interface.INotifications` (`self.Mission HUD Ref`) (`KismetTextLibrary.Conv_IntToText` (`self.DroneTImer`))) ; Sending to MissionHUD
    )))

(event `InputAxis|MoveRight` :overrideparent false
  (params (AxisValue :type "Float (single-precision)"))
  ;[1 1 1] Drone Movement (W,A,S,D)
  (`self.AddMovementInput` (`KismetMathLibrary.GetRightVector` (`KismetMathLibrary.MakeRotator` 0.0 0.0 (.yaw (`self.GetControlRotation`)))) (* AxisValue 0.3)))

(fn `UserConstructionScript`)