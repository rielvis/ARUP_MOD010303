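; Stealth hazard laser beam actor that raises an alarm when the player's ThirdPersonCharacter overlaps it.
; An enum picks the behavior on BeginPlay: type 1 blinks visibility and collision on a fixed delay loop, while type 2 moves via InterpToMovement.
; Beam overlap reports an "Alarm"-tagged noise event at the actor's root, with the character as instigator, for AI hearing.
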(event `self.ReceiveBeginPlay`
  (switch `/Game/Stealth/ELaserBeamType` (`self.LaserBeamType`)
    (:`NewEnumerator1`
      (`self.Event_LaserBeamType1_Active`))
    (:`NewEnumerator0`
      (`self.Event_LaserBeamType2_Active`))))

(event `Event_LaserBeamType1_Active`
  (bind _sm_laserbeam (`self.SM_LaserBeam`))
  (bind _sm_laserbeam_2 (`self.SM_LaserBeam`))
  ;[1 1 1] Type1_ LAser Beam Toggle on/off Every provided seconds (Delay)
  (`ActorComponent.SetActive` (`self.InterpToMovement`) false false)
  (`SceneComponent.SetHiddenInGame` _sm_laserbeam_2 true false :!label _label)
  (`PrimitiveComponent.SetCollisionEnabled` _sm_laserbeam_2 "NoCollision")
  (`KismetSystemLibrary.Delay` 3.0)
  (`SceneComponent.SetHiddenInGame` _sm_laserbeam false false)
  (`PrimitiveComponent.SetCollisionEnabled` _sm_laserbeam "QueryOnly")
  (`KismetSystemLibrary.Delay` 3.0)
  (`KismetSystemLibrary.PrintString` "Hello")
  (goto _label))

(event `Event_LaserBeamType2_Active`
  ;[1 1 1] Type2_ Laser Beam moving between two points using InterpToMovement components
  (`ActorComponent.SetActive` (`self.InterpToMovement`) true false))

(event `self.SM_LaserBeam.OnComponentBeginOverlap`
  (params (OverlappedComponent :type "PrimitiveComponent Object Reference") (OtherActor :type "Actor Object Reference") (OtherComp :type "PrimitiveComponent Object Reference") (OtherBodyIndex :type Integer) (bFromSweep :type Boolean) (SweepResult :type "HitResult Structure (by ref)"))
  ;[1 1 1] Set Alarm_On collision with laser beam set alarm
  (bind _asthird_person_character (cast `/Game/Stealth/ThirdPersonBP/Blueprints/ThirdPersonCharacter` OtherActor))
  (`AISense_Hearing.ReportNoiseEvent` (`SceneComponent.K2_GetComponentLocation` (`self.DefaultSceneRoot`)) 1.0 _asthird_person_character 1500.0 "Alarm")
  (`KismetSystemLibrary.PrintString` "Laser Beam_ Set Alarm" true true (struct :`R` 1.0 :`B` 0.012164 :`A` 1.0)))

(fn `UserConstructionScript`)